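; BP_TestA is a scratch test actor for trying out basic Blueprint features.
; The construction script writes MyName into a TextRender component, and Tick prints DeltaSeconds on screen every frame.
; BeginPlay and ActorBeginOverlap are empty.
; The remaining nodes are disconnected experiments with delays, a looping print, a traffic-light enum, structs, visibility, arrays and lookups, and never execute.
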(event EventBeginPlay)

(event Collision|EventActorBeginOverlap
  (params (OtherActor :type Actor%20Object%20Reference)))

(event EventTick
  (params (DeltaSeconds :type Float%20%28single-precision%29))
  (Development|PrintString (Utilities|String|ToString(Float) DeltaSeconds) true false "(R=0.325244,G=1.000000,B=0.900129,A=1.000000)" DeltaSeconds))

(fn ConstructionScript
  (Rendering|Components|TextRender|SetText (Variables|Default|GetTextRender) (Utilities|Text|FormatText "My name is {Name}" (Variables|Test|GetMy_name))))